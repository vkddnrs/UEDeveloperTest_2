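; BP_ky_cutter3 is a magic FX spawner actor that launches six cutter effects at once on BeginPlay.
; SpawnCutter spawns a BP_ky_cutter2 at each of six point component transforms, passing on color, loop flag and shot speed.
; The color is also pushed directly into each spawned effect's "color" vector parameter.
; After a short delay the spawner destroys itself, regardless of the loop flag.
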(event EventBeginPlay
  ;[1 1 1] fx1 spawn
  (CallFunction|SpawnCutter (Transformation|GetWorldTransform (Variables|Default|Getpoint1)) (Variables|Default|Getcolor) (Variables|Default|GetisLoop) (Variables|Default|GetshotSpeed))
  ;[1 1 1] fx2 spawn
  (CallFunction|SpawnCutter (Transformation|GetWorldTransform (Variables|Default|Getpoint2)) (Variables|Default|Getcolor) (Variables|Default|GetisLoop) (Variables|Default|GetshotSpeed))
  ;[1 1 1] fx3 spawn
  (CallFunction|SpawnCutter (Transformation|GetWorldTransform (Variables|Default|Getpoint3)) (Variables|Default|Getcolor) (Variables|Default|GetisLoop) (Variables|Default|GetshotSpeed))
  ;[1 1 1] fx4 spawn
  (CallFunction|SpawnCutter (Transformation|GetWorldTransform (Variables|Default|Getpoint4)) (Variables|Default|Getcolor) (Variables|Default|GetisLoop) (Variables|Default|GetshotSpeed))
  ;[1 1 1] fx5 spawn
  (CallFunction|SpawnCutter (Transformation|GetWorldTransform (Variables|Default|Getpoint5)) (Variables|Default|Getcolor) (Variables|Default|GetisLoop) (Variables|Default|GetshotSpeed))
  ;[1 1 1] fx6 spawn
  (CallFunction|SpawnCutter (Transformation|GetWorldTransform (Variables|Default|Getpoint6)) (Variables|Default|Getcolor) (Variables|Default|GetisLoop) (Variables|Default|GetshotSpeed))
  (Utilities|FlowControl|Delay 4.0)
  (Actor|DestroyActor))

(fn ConstructionScript)

(fn SpawnCutter
  (params (transform :type Transform) (color :type Linear%20Color%20Structure) (loop :type Boolean) (speed :type Float%20%28single-precision%29))
  ;[1 1 1] fx spawn
  (bind _returnvalue (Game|SpawnActorfromClass "/Game/AdvancedMagicFX13/Blueprints/BP_ky_cutter2.BP_ky_cutter2_C" transform "Undefined" 0 0))
  ;[1 1 1] color control
  (Effects|Components|ParticleSystem|SetVectorParameter (Variables|/Game/AdvancedMagicFX13/Blueprints/BP_ky_cutter2.BP_ky_cutter2_C|GetFX _returnvalue) "color" (Math|Conversions|ToVector(LinearColor) color))
  ;[1 1 1] color set
  (Variables|/Game/AdvancedMagicFX13/Blueprints/BP_ky_cutter2.BP_ky_cutter2_C|Setcolor _returnvalue color)
  ;[1 1 1] loop flg set
  (Variables|/Game/AdvancedMagicFX13/Blueprints/BP_ky_cutter2.BP_ky_cutter2_C|SetisLoop _returnvalue loop)
  ;[1 1 1] move speed set
  (Variables|/Game/AdvancedMagicFX13/Blueprints/BP_ky_cutter2.BP_ky_cutter2_C|SetshotSpeed _returnvalue speed))